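; Player pawn for the Lindwyrm Roll minigame: a gnome with a per-player color that moves, jumps, and carries gold and rings.
; Input moves it relative to the minigame's scene-capture camera, while Tick fakes gravity using a Z velocity and downward ground trace.
; Stuns block movement and gravity.
; Wyrm hits trigger a tweened squash and check distance bands for gold loss, though SignOfInteger reduces each band's amount to one.
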(event Custom|is%20moving?
  ;[1 1 1] Running particles
  (if (not (Utilities|Operators|EqualEqual :A (Transformation|GetComponentVelocity (Variables|Default|GetCollition_Capsule)) :ErrorTolerance 2.0))
    (AddComponent|AddNiagaraComponent false (Math|Transform|MakeTransform "0.000000,0.000000,-60.000000" "0, 0, 0" "1.000000,1.000000,1.000000"))))

(event Custom|GnomeHit
  (bind _value (|TweenVector (Transformation|GetActorScale3D) "2.000000,2.000000,0.010000" 0.1 "InOutQuad")
    (:ApplyEasing
      (Transformation|SetActorScale3D _value))
    (:OnComplete
      (Utilities|FlowControl|Delay 0.7)
      (bind _value_2 (|TweenVector "2.000000,2.000000,0.100000" "1.000000,1.000000,1.000000" 2.0 "OutElastic")
        (:ApplyEasing
          (Transformation|SetActorScale3D _value_2))))))

(event Input|EnhancedActionEvents|EnhancedInputActionIA_Button1
  (params (ActionValue :type Boolean) (ElapsedSeconds :type Float%20%28double-precision%29) (TriggeredSeconds :type Float%20%28double-precision%29) (InputAction :type Input%20Action%20Object%20Reference :default "/MinigameCore/Input/IA_Button1.IA_Button1"))
  ;[0.1436 0.0916 1] Jumping
  (CallFunction|Jump))

(event Input|EnhancedActionEvents|EnhancedInputActionIA_Movement
  (params (ActionValue :type Vector%202D%20Structure) (ElapsedSeconds :type Float%20%28double-precision%29) (TriggeredSeconds :type Float%20%28double-precision%29) (InputAction :type Input%20Action%20Object%20Reference :default "/MinigameCore/Input/IA_Movement.IA_Movement"))
  ;[0.1232 1 0.3635] WASD Movment
  (:Triggered
    (CallFunction|Move ActionValue))
  (:Completed
    (Variables|Default|SetAlpha 0.0)))

(event EventBeginPlay
  ;[1 1 1] Start up values
  (bind _returnvalue (Actor|GetActorOfClass "/MinigameCore/Game/BP_MinigameCapture.BP_MinigameCapture_C"))
  (Variables|Default|SetCamera _returnvalue)
  (Variables|Default|SetGoldAmount 20)
  (CallFunction|SetupPlayerColors))

(event EventTick
  (params (DeltaSeconds :type Float%20%28single-precision%29))
  (bind _collition_capsule (Variables|Default|GetCollition_Capsule))
  (bind _returnvalue (Transformation|GetWorldLocation _collition_capsule))
  ;[1 1 1] Fake gravity
  (CallFunction|IsMoving?)
  (if (Variables|Default|GetisRestricted)
    (if (<= (Variables|Default|GetStunTime) 0.0)
      (bind _returnvalue_2 (Collision|LineTraceByChannel _returnvalue (+ _returnvalue "0.000000,0.000000,-95.000000") "TraceTypeQuery1" false 0 "ForOneFrame"))
      (Variables|Default|SetCanJump (and (< (Variables|Default|GetZVelocity) 0.0) _returnvalue_2))
      (Transformation|AddWorldOffset (Variables|Default|GetCollition_Capsule) (Math|Vector|MakeVector 0.0 0.0 (Math|Float|SelectFloat 0.0 (Variables|Default|GetZVelocity) (and (< (Variables|Default|GetZVelocity) 0.0) _returnvalue_2))) true false)
      (bind _output_get (Variables|Default|SetZVelocity (- (Math|Float|Clamp(Float) (stale _output_get) -9e+02 9e+02) 1.0)))
      (else
        (Utilities|FlowControl|Delay (Variables|Default|GetStunTime))
        (Variables|Default|SetStunTime 0.0)
        (Variables|Default|SetZVelocity 0.0)))))

(event Input|KeyboardEvents|F
  (params (Key :type Key%20Structure :default "None"))
  (:Pressed
    (for _index (range 0 3)
      (Class|MinigameBase|ReadyPlayer (Variables|Default|GetMinigame) _index false))))

(fn ConstructionScript
  (Variables|/Game/LindwyrmRoll/Blueprints/Props/BP_RingHolder.BP_RingHolder_C|SetRingSpline (Variables|Default|GetBP_RingHolder) (Variables|Default|GetRingHolder)))

(fn GetHitandGiveGold
  (params (wyrm%20 :type BP%20Rolling%20Wyrm%20Object%20Reference))
  (bind _returnvalue (Transformation|GetDistanceTo wyrm%20))
  (bind _returnvalue_2 (Class|KismetMathLibrary|SignOfInteger 5))
  (bind _returnvalue_3 (Class|KismetMathLibrary|SignOfInteger 15))
  (bind _returnvalue_4 (Class|KismetMathLibrary|SignOfInteger 10))
  (bind _returnvalue_5 (Math|Float|Truncate _returnvalue))
  (CallFunction|GnomeHit)
  (if (< _returnvalue_5 40)
    (Variables|Default|SetGoldAmount (- (Variables|Default|GetGoldAmount) _returnvalue_3))
    (Development|PrintString "MAX hit")
    (return _returnvalue_3)
    (elif (< _returnvalue_5 75)
      (Variables|Default|SetGoldAmount (- (Variables|Default|GetGoldAmount) _returnvalue_4))
      (Development|PrintString "Medium far hit")
      (return _returnvalue_4)
      (elif (<= _returnvalue_5 90)
        (Variables|Default|SetGoldAmount (- (Variables|Default|GetGoldAmount) _returnvalue_2))
        (Development|PrintString "FAR but close")
        (return _returnvalue_2)
        (else
          (Development|PrintString "Not Close")
          (return 0))))))

(fn StunGnome
  (params (Duration :type Float%20%28double-precision%29))
  (if (> (Variables|Default|GetStunTime) 0.0)
    _
    (else
      (Variables|Default|SetStunTime 0.5)))
  (return))

(fn TakeGold
  (params (amount :type Integer))
  (if (> amount (Variables|Default|GetGoldAmount))
    (Variables|Default|SetGoldAmount 0)
    (else
      (Variables|Default|SetGoldAmount (- (Variables|Default|GetGoldAmount) amount)))))

(fn RemoveRings
  (params (AmountToRemove :type Integer))
  (bind _difference (Default|SetAmountOfRings (Variables|Default|GetBP_RingHolder) (Math|Integer|Clamp(Integer) (- (Variables|/Game/LindwyrmRoll/Blueprints/Props/BP_RingHolder.BP_RingHolder_C|GetCurrentRings (Variables|Default|GetBP_RingHolder)) AmountToRemove) 0 100)))
  (return _difference))

(fn SetupPlayerColors
  (bind _returnvalue (Rendering|Material|CreateDynamicMaterialInstance (Variables|Default|GetGnomeMesh) 0 "/Game/LindwyrmRoll/Characters/Gnome/MI_Gnome.MI_Gnome" "None" :!class /Script/Engine.PrimitiveComponent))
  (bind _asbp_lindwyrm_roll_gamemode (Utilities|Casting|CastToBP_LindwyrmRollGamemode (Game|GetGameMode)))
  (Rendering|Material|SetVectorParameterValue _returnvalue "PlayerColor" (Utilities|Array|Get(acopy) (Variables|/Game/LindwyrmRoll/Blueprints/Gamemanagers/BP_LindwyrmRollGamemode.BP_LindwyrmRollGamemode_C|GetPlayerColors _asbp_lindwyrm_roll_gamemode) (Variables|Default|GetPlayerNumber)) :!class /Script/Engine.MaterialInstanceDynamic))

(fn Move
  (params (InVec :type Vector%202D%20Structure))
  (bind (_x _y) (Math|Vector2D|BreakVector2D InVec))
  (bind _movespeed (Variables|Default|GetMoveSpeed))
  (bind _camera (Variables|Default|GetCamera))
  (bind _scenecapture (Variables|/Script/MinigameCore.MinigameCapture|GetSceneCapture _camera))
  (bind _returnvalue (Math|Vector|GetForwardVector _scenecapture))
  (bind _returnvalue_2 (Math|Vector|GetRightVector _scenecapture))
  (bind _returnvalue_3 (* _returnvalue_2 _movespeed _x))
  (bind _returnvalue_4 (* _returnvalue _movespeed _y))
  (bind _returnvalue_5 (+ _returnvalue_3 _returnvalue_4))
  (bind _returnvalue_6 (Math|Vector|MakeVector (.x _returnvalue_5) (.y _returnvalue_5) (.z _returnvalue_5)))
  (CallFunction|MoveInternal (Math|Vector2D|MakeVector2D (.x _returnvalue_6) (.y _returnvalue_6))))

(fn Jump
  (Animation|Montage|MontagePlay (Components|SkeletalMesh|GetAnimInstance (Variables|Default|GetGnomeMesh)) "/BashAssets/Character/Modular/Animations/AM_Jump.AM_Jump" 1.0 "MontageLength" 0.0 true)
  (if (Variables|Default|GetCanJump)
    (AddComponent|AddNiagaraComponent false (Math|Transform|MakeTransform "0, 0, 0" "0, 0, 0" "0.500000,0.500000,0.500000"))
    (Variables|Default|SetZVelocity 2e+01)
    (Variables|Default|SetCanJump false)))

(fn MoveInternal
  (params (Direction :type Vector%202D%20Structure))
  (if (<= (Variables|Default|GetStunTime) 0.0)
    (Pawn|Input|AddMovementInput (Math|Vector|MakeVector (.x Direction) (.y Direction) 0.0) 1.0 false)
    (Transformation|SetActorRotation (Math|Rotator|MakeRotator 0.0 0.0 (Utilities|RotateMacro (Math|Rotator|FindLookatRotation (Math|Vector|MakeVector 0.0 0.0 0.0) (Math|Vector|MakeVector (.x Direction) (.y Direction) 0.0)) 3.0)))))