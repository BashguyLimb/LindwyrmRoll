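; Player-controlled gnome for a Lindwyrm minigame, with movement, jumping, a gold purse and a stun state.
; Movement is relative to the minigame capture camera and turns the gnome through a rotate macro, while Tick fakes gravity using a Z velocity and ground trace.
; Hits check distance tiers to the wyrm, but SignOfInteger reduces every payout to one gold.
; StunGnome ignores Duration, and nothing visible clears the movement-blocking StunTime.
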(event Input|EnhancedActionEvents|EnhancedInputActionIA_Button1
  (params (ActionValue :type Boolean) (ElapsedSeconds :type Float%20%28double-precision%29) (TriggeredSeconds :type Float%20%28double-precision%29) (InputAction :type Input%20Action%20Object%20Reference :default "/MinigameCore/Input/IA_Button1.IA_Button1"))
  ;[0.1436 0.0916 1] Jumping
  (:Started
    (if (Variables|Default|GetCanJump)
      (Variables|Default|SetZVelocity 2e+01)
      (Variables|Default|SetCanJump false))))

(event Input|EnhancedActionEvents|EnhancedInputActionIA_Movement
  (params (ActionValue :type Vector%202D%20Structure) (ElapsedSeconds :type Float%20%28double-precision%29) (TriggeredSeconds :type Float%20%28double-precision%29) (InputAction :type Input%20Action%20Object%20Reference :default "/MinigameCore/Input/IA_Movement.IA_Movement"))
  (bind (_x _y) (Math|Vector2D|BreakVector2D ActionValue))
  (bind _camera (Variables|Default|GetCamera))
  (bind _movespeed (Variables|Default|GetMoveSpeed))
  (bind _scenecapture (Variables|/Script/MinigameCore.MinigameCapture|GetSceneCapture _camera))
  (bind _returnvalue (Math|Vector|GetForwardVector _scenecapture))
  (bind _returnvalue_2 (Math|Vector|GetRightVector _scenecapture))
  (bind _returnvalue_3 (* _returnvalue_2 _movespeed _x))
  (bind _returnvalue_4 (* _returnvalue _movespeed _y))
  (bind _returnvalue_5 (+ _returnvalue_3 _returnvalue_4))
  ;[0.1232 1 0.3635] WASD Movment
  (:Triggered
    (if (== (Variables|Default|GetStunTime) 0.0)
      (Pawn|Input|AddMovementInput (Math|Vector|MakeVector (.x _returnvalue_5) (.y _returnvalue_5) 0.0) 1.0 false)
      (Transformation|SetActorRotation (Math|Rotator|MakeRotator 0.0 0.0 (Utilities|RotateMacro (Math|Rotator|FindLookatRotation (Math|Vector|MakeVector 0.0 0.0 0.0) (Math|Vector|MakeVector (.x _returnvalue_5) (.y _returnvalue_5) (.z _returnvalue_5))) 0.85)))))
  (:Completed
    (Variables|Default|SetAlpha 0.0)))

(event EventTick
  (params (DeltaSeconds :type Float%20%28single-precision%29))
  (bind _collition_capsule (Variables|Default|GetCollition_Capsule))
  (bind _returnvalue (Transformation|GetWorldLocation _collition_capsule))
  ;[1 1 1] Fake gravity
  (bind _returnvalue_2 (Collision|LineTraceByChannel _returnvalue (+ _returnvalue "0.000000,0.000000,-65.000000") "TraceTypeQuery1" false 0 "ForOneFrame"))
  (Development|PrintString (Utilities|String|ToString(Float) (Variables|Default|GetZVelocity)))
  (Variables|Default|SetCanJump (and (< (Variables|Default|GetZVelocity) 0.0) _returnvalue_2))
  (Transformation|AddWorldOffset (Variables|Default|GetCollition_Capsule) (Math|Vector|MakeVector 0.0 0.0 (Math|Float|SelectFloat 0.0 (Variables|Default|GetZVelocity) (and (< (Variables|Default|GetZVelocity) 0.0) _returnvalue_2))) false false)
  (bind _output_get (Variables|Default|SetZVelocity (- (Math|Float|Clamp(Float) (stale _output_get) -9e+02 9e+02) 1.0))))

(event EventOnReset
  ;[1 1 1] Clean up
  (Actor|DestroyActor))

(event EventBeginPlay
  ;[1 1 1] Start up values
  (bind _returnvalue (Actor|GetActorOfClass "/MinigameCore/BP_MinigameCapture.BP_MinigameCapture_C"))
  (Variables|Default|SetCamera _returnvalue)
  (Variables|Default|SetGoldAmount 20))

(fn ConstructionScript)

(fn GetHitandGiveGold
  (params (wyrm%20 :type BP%20Rolling%20Wyrm%20Object%20Reference))
  (bind _returnvalue (Transformation|GetDistanceTo wyrm%20))
  (bind _returnvalue_2 (Class|KismetMathLibrary|SignOfInteger 5))
  (bind _returnvalue_3 (Class|KismetMathLibrary|SignOfInteger 15))
  (bind _returnvalue_4 (Class|KismetMathLibrary|SignOfInteger 10))
  (bind _returnvalue_5 (Math|Float|Truncate _returnvalue))
  (if (< _returnvalue_5 40)
    (Variables|Default|SetGoldAmount (- (Variables|Default|GetGoldAmount) _returnvalue_3))
    (Development|PrintString "MAX hit")
    (return _returnvalue_3)
    (elif (< _returnvalue_5 75)
      (Variables|Default|SetGoldAmount (- (Variables|Default|GetGoldAmount) _returnvalue_4))
      (Development|PrintString "Medium far hit")
      (return _returnvalue_4)
      (elif (<= _returnvalue_5 90)
        (Variables|Default|SetGoldAmount (- (Variables|Default|GetGoldAmount) _returnvalue_2))
        (Development|PrintString "FAR but close")
        (return _returnvalue_2)
        (else
          (Development|PrintString "Not Close")
          (return 0))))))

(fn StunGnome
  (params (Duration :type Float%20%28double-precision%29))
  (if (> (Variables|Default|GetStunTime) 0.0)
    _
    (else
      (Variables|Default|SetStunTime 0.5)))
  (return))

(fn TakeGold
  (params (amount :type Integer))
  (if (> amount (Variables|Default|GetGoldAmount))
    (Variables|Default|SetGoldAmount 0)
    (else
      (Variables|Default|SetGoldAmount (- (Variables|Default|GetGoldAmount) amount)))))