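; Player in the LindwyrmRoll game that aims and throws a rolling Lindwyrm.
; Movement input turns a clamped aim angle, and the action button launches a single reused BP_RollingWyrm along it, or boosts it once per throw while it cannot fire.
; The held wyrm mesh shows only when a throw is available.
; BeginPlay picks a random color index for the wyrm materials and repositions the character mesh for right-side players.
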(event Input|EnhancedActionEvents|EnhancedInputActionIA_Movement
  (params (ActionValue :type Vector%202D%20Structure) (ElapsedSeconds :type Float%20%28double-precision%29) (TriggeredSeconds :type Float%20%28double-precision%29) (InputAction :type Input%20Action%20Object%20Reference :default "/MinigameCore/Input/IA_Movement.IA_Movement"))
  (Variables|Default|SetCurrent%20Rotation (Math|Float|Clamp(Float) (+ (* (Utilities|Time|GetWorldDeltaSeconds) (Variables|Default|GetRotationSpeed) (.x ActionValue)) (Variables|Default|GetCurrent%20Rotation)) (* (Variables|Default|GetMaxRotation) -1.0) (Variables|Default|GetMaxRotation))))

(event Input|EnhancedActionEvents|EnhancedInputActionIA_Button1
  (params (ActionValue :type Boolean) (ElapsedSeconds :type Float%20%28double-precision%29) (TriggeredSeconds :type Float%20%28double-precision%29) (InputAction :type Input%20Action%20Object%20Reference :default "/MinigameCore/Input/IA_Button1.IA_Button1"))
  (:Started
    (CallFunction|ActionPressed)))

(event EventBeginPlay
  (Variables|Default|SetMaterialIndex (Math|Random|RandomInteger 4))
  (CallFunction|SetPlayerColor (Variables|Default|GetLindwyrmPlayer))
  (bind _output_get (Variables|Default|SetonRight (> (.y (Transformation|GetWorldLocation (Variables|Default|GetPlayer))) 8e+02)))
  (if _output_get
    (Transformation|SetWorldLocation (Variables|Default|GetPlayer) "-4910.983513,1250.000000,480.618475" false false)))

(event EventTick
  (params (DeltaSeconds :type Float%20%28single-precision%29))
  (bind _lindwyrmplayer (Variables|Default|GetLindwyrmPlayer))
  (bind _spawnedwyrm (Variables|Default|GetSpawnedWyrm)
    (:then
      (if (Variables|/Game/LindwyrmRoll/Blueprints/RollingWyrm/BP_RollingWyrm.BP_RollingWyrm_C|GetCanFire _spawnedwyrm)
        (Rendering|SetVisibility _lindwyrmplayer true false :!label _label)
        (else
          (Rendering|SetVisibility _lindwyrmplayer false false))))
    (:else
      (goto _label))))

(fn ConstructionScript)

(fn ThrowWyrm
  (bind _spawnpoint (Variables|Default|GetSpawnPoint))
  (bind _spawnpoint_2 (Variables|Default|GetSpawnPoint))
  (Animation|Montage|MontagePlay (Components|SkeletalMesh|GetAnimInstance (Variables|Default|GetPlayer)) "/Game/LindwyrmRoll/Characters/Player/ModChara_Point_Montage.ModChara_Point_Montage" 1.0 "MontageLength" 0.0 true)
  (bind _spawnedwyrm (Variables|Default|GetSpawnedWyrm)
    (:then
      (Transformation|SetActorTransform _spawnedwyrm (Math|Transform|MakeTransform (Transformation|GetWorldLocation _spawnpoint_2) (Transformation|GetWorldRotation _spawnpoint_2) (Variables|Default|GetWyrmScale)))
      (Physics|SetPhysicsLinearVelocity (Variables|/Game/LindwyrmRoll/Blueprints/RollingWyrm/BP_RollingWyrm.BP_RollingWyrm_C|GetSphereHitbox _spawnedwyrm) "0, 0, 0" false "None"))
    (:else
      (bind _returnvalue (Game|SpawnActorfromClass "/Game/LindwyrmRoll/Blueprints/RollingWyrm/BP_RollingWyrm.BP_RollingWyrm_C" (Math|Transform|MakeTransform (Transformation|GetWorldLocation _spawnpoint) (Transformation|GetWorldRotation _spawnpoint) (Variables|Default|GetWyrmScale)) "Undefined" "OverrideRootScale" 0 0))
      (Variables|/Game/LindwyrmRoll/Blueprints/RollingWyrm/BP_RollingWyrm.BP_RollingWyrm_C|SetPlayerOwner _returnvalue self)
      (CallFunction|SetPlayerColor (Variables|/Game/LindwyrmRoll/Blueprints/RollingWyrm/BP_RollingWyrm.BP_RollingWyrm_C|GetLindwyrm _returnvalue))
      (bind _output_get (Variables|Default|SetSpawnedWyrm _returnvalue))))
  (Default|LaunchWyrm _output_get (Math|Vector|RotateVectorAroundAxis (Math|Vector|GetForwardVector (Variables|Default|GetSpawnPoint)) (Variables|Default|GetCurrent%20Rotation) "0.000000,0.000000,1.000000"))
  (bind _asbp_lindwyrm_roll_gamemode (Utilities|Casting|CastToBP_LindwyrmRollGamemode (Game|GetGameMode))))

(fn ActionPressed
  (bind _spawnedwyrm (Variables|Default|GetSpawnedWyrm)
    (:then
      (if (Variables|/Game/LindwyrmRoll/Blueprints/RollingWyrm/BP_RollingWyrm.BP_RollingWyrm_C|GetCanFire _spawnedwyrm)
        (CallFunction|ThrowWyrm :!label _label)
        (goto _label_2 Reset)
        (else
          (Utilities|FlowControl|DoOnce false :!label _label_2
            (:Completed
              (Default|BoostWyrm (Variables|Default|GetSpawnedWyrm)))))))
    (:else
      (goto _label))))

(fn SetPlayerColor
  (params (SkeletalMesh :type Skeletal%20Mesh%20Component%20Object%20Reference))
  (bind _returnvalue (Rendering|Material|CreateDynamicMaterialInstance SkeletalMesh 0 "/Game/LindwyrmRoll/Characters/Lindwyrm/MI_Lindwyrm.MI_Lindwyrm" "None" :!class /Script/Engine.PrimitiveComponent))
  (Rendering|Material|SetScalarParameterValue _returnvalue "Index" (Math|Conversions|ToFloat(Integer) (Variables|Default|GetMaterialIndex)) :!class /Script/Engine.MaterialInstanceDynamic)
  (for _index (range 0 3)
    (Rendering|Material|SetScalarParameterValueonMaterials (Variables|Default|GetLindwyrmPlayer) "Index" (Math|Conversions|ToFloat(Integer) (Variables|Default|GetMaterialIndex)))))