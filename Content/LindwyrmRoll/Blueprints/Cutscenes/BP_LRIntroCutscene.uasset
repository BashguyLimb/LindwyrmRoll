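; Intro cutscene Blueprint for LindwyrmRoll that puts the level's gnome players into the cutscene's Level Sequence.
; InitializeLevelSequence gathers all BP_GnomePlayer actors and binds the first two, when valid, to the Gnome1 and Gnome2 binding tags on the given sequence actor.
; Gnome roles follow the order GetAllActorsOfClass returns, and the bindings replace those from the sequence asset.
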(fn InitializeLevelSequence
  (params (SequenceActor :type Level%20Sequence%20Actor%20Object%20Reference))
  (bind _outactors (Actor|GetAllActorsOfClass SequenceActor "/Game/LindwyrmRoll/Blueprints/GnomePlayer/BP_GnomePlayer.BP_GnomePlayer_C"))
  (LocalVariables|SetGnomes _outactors)
  (Utilities|FlowControl|Sequence
    (:then_0
      (Utilities|IsValid (Utilities|Array|Get(acopy) (LocalVariables|GetGnomes))
        (:Is%20Valid
          (Class|LevelSequenceActor|SetBindingbyTag SequenceActor "Gnome1" (Utilities|Array|MakeArray (Utilities|Array|Get(acopy) (LocalVariables|GetGnomes))) false))))
    (:then_1
      (Utilities|IsValid (Utilities|Array|Get(acopy) (LocalVariables|GetGnomes) 1)
        (:Is%20Valid
          (Class|LevelSequenceActor|SetBindingbyTag SequenceActor "Gnome2" (Utilities|Array|MakeArray (Utilities|Array|Get(acopy) (LocalVariables|GetGnomes) 1)) false))))))