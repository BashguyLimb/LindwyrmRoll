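; Camera shake handler component that jitters an affected component's relative location for a requested duration, amplitude and frequency.
; BeginPlay binds a start-shake event, which caches the starting transform, stores the parameters and resets the timer.
; Tick offsets location with phase-shifted 1D Perlin noise per axis, keeping rotation and scale.
; Tick never checks IsShaking, reapplying the cached transform every frame once the duration expires.
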(event Custom|CustomEvent
  (params (Duration :type Float%20%28double-precision%29) (Amplitude :type Vector) (Frequency :type Float%20%28double-precision%29))
  (Utilities|FlowControl|Sequence
    (:then_0
      (Variables|Default|SetStartPos (Transformation|GetRelativeTransform (Variables|Default|GetAffectedComponent))))
    (:then_1
      (Variables|Default|SetShakeDuration Duration))
    (:then_2
      (Variables|Default|SetShakeAmplitude Amplitude))
    (:then_3
      (Variables|Default|SetShakeFrequency Frequency))
    (:then_4
      (Variables|Default|SetShakeTimeElapsed 0.0)
      (Variables|Default|SetIsShaking true))))

(event EventBeginPlay
  (EventDispatchers|BindEventtoStartShake (delegate Custom|CustomEvent)))

(event EventTick
  (params (DeltaSeconds :type Float%20%28single-precision%29))
  (bind _startpos (Variables|Default|GetStartPos))
  (Variables|Default|SetShakeTimeElapsed (+ DeltaSeconds (Variables|Default|GetShakeTimeElapsed)))
  (if (> (Variables|Default|GetShakeTimeElapsed) (Variables|Default|GetShakeDuration))
    (Variables|Default|SetIsShaking false)
    (Transformation|SetRelativeTransform (Variables|Default|GetAffectedComponent) (Variables|Default|GetStartPos) false false)
    (else
      (Transformation|SetRelativeTransform (Variables|Default|GetAffectedComponent) (Math|Transform|MakeTransform (+ (* (Math|Vector|MakeVector (Class|KismetMathLibrary|PerlinNoise1D (* (Variables|Default|GetShakeTimeElapsed) (Variables|Default|GetShakeFrequency))) (Class|KismetMathLibrary|PerlinNoise1D (+ (* (Variables|Default|GetShakeTimeElapsed) (Variables|Default|GetShakeFrequency)) 2e+01)) (Class|KismetMathLibrary|PerlinNoise1D (+ (* (Variables|Default|GetShakeTimeElapsed) (Variables|Default|GetShakeFrequency)) 4e+01))) (Variables|Default|GetShakeAmplitude)) (.location _startpos)) (.rotation _startpos) (.scale _startpos)) false false))))