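; Physics-driven rolling lindwyrm projectile that rams gnome players, stunning them, taking their rings and transferring points to the rollers through the gamemode.
; LaunchWyrm fires the sphere hitbox by impulse and starts a delayed scale tween, while BoostWyrm pushes along horizontal velocity when allowed.
; Tick spins the model pivot from velocity and re-enables firing after a timeout.
; Camera shake and sounds accompany hits; ReturntoStart tweens toward the owner's rotation.
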(event OnComponentBeginOverlap(SphereHitbox)
  (params (OverlappedComponent :type Primitive%20Component%20Object%20Reference) (OtherActor :type Actor%20Object%20Reference) (OtherComp :type Primitive%20Component%20Object%20Reference) (OtherBodyIndex :type Integer) (bFromSweep :type Boolean) (SweepResult :type Hit%20Result%20Structure%20%28by%20ref%29))
  ;[1 0 0.01848] Collisions
  (Variables|Default|Sethit true)
  ;;[0 0.1395 1] Gnome Collisions
  (bind _asbp_gnome_player (Utilities|Casting|CastToBP_GnomePlayer OtherActor))
  (Default|GetHitandGiveGold _asbp_gnome_player)
  (Default|StunGnome _asbp_gnome_player 0.0)
  (bind _amountremoved (Default|RemoveRings _asbp_gnome_player 3))
  (bind _ringsadded (CallFunction|AddRings _amountremoved))
  (bind _asbp_lindwyrm_roll_gamemode (Utilities|Casting|CastToBP_LindwyrmRollGamemode (Game|GetGameMode)))
  (Default|TransferPointstoRollers _asbp_lindwyrm_roll_gamemode _ringsadded)
  (Class|MinigameCapture|ApplyCameraShake (Class|MinigameBase|GetCamera _asbp_lindwyrm_roll_gamemode) 5.0 0.2)
  (Audio|PlaySound2D "/Game/LindwyrmRoll/Sound/SW_desk-thud-106752.SW_desk-thud-106752" 1.0 1.0 0.0 0 0)
  (Audio|PlaySound2D "/Game/LindwyrmRoll/Sound/CoinFall1.CoinFall1" 1.0 1.0 0.0 0 0)
  (Variables|Default|SetCanBoost false))

(event OnComponentEndOverlap(SphereHitbox)
  (params (OverlappedComponent :type Primitive%20Component%20Object%20Reference) (OtherActor :type Actor%20Object%20Reference) (OtherComp :type Primitive%20Component%20Object%20Reference) (OtherBodyIndex :type Integer))
  ;[1 0 0.01848] Collisions
  (Variables|Default|SetCanBoost true))

(event Custom|Return%20to%20Start
  (bind _playerowner (Variables|Default|GetPlayerOwner))
  (Variables|Default|SetStartTweenRot (Transformation|GetActorRotation))
  (Variables|Default|SetStartTweenPos (Transformation|GetActorLocation))
  (Development|PrintString "return to start!!")
  (bind _value (|TweenFloat 0.0 1.0 1.0 "InOutQuad")
    (:ApplyEasing
      (Transformation|SetActorLocation (Math|Vector|Lerp(Vector) (Variables|Default|GetStartTweenPos) (Transformation|GetActorLocation _playerowner) 0.0) false false)
      (Transformation|SetActorRotation (Math|Rotator|Lerp(Rotator) (Variables|Default|GetStartTweenRot) (Transformation|GetActorRotation _playerowner) _value true))
      (if (Variables|Default|GetIsRolling)
        (Utilities|FlowControl|Delay 1.5)
        (Actor|DestroyActor)))
    (:OnComplete
      (Variables|Default|SetCanFire true))))

(event Custom|Tween%20Scale
  (Utilities|FlowControl|Sequence
    (:then_0
      (bind _scale_tween (Variables|Default|GetScale%20Tween)
        (:then
          (Class|FCTweenBPAction|Stop _scale_tween))
        (:else)))
    (:then_1
      (Utilities|FlowControl|Delay 2.5)
      (bind (_asynctaskproxy _value) (|TweenVector (Transformation|GetActorScale3D) "0, 0, 0" 1.0 "Linear")
        (:then
          (Variables|Default|SetScale%20Tween _asynctaskproxy))
        (:ApplyEasing
          (Transformation|SetActorScale3D _value))))))

(event EventBeginPlay
  (Audio|SpawnSoundAttached "/Game/LindwyrmRoll/Sound/SW_earth-rumble-6953.SW_earth-rumble-6953" (Variables|Default|GetSphereHitbox) "None" "0, 0, 0" "0, 0, 0" "SnapToTarget" false 1.0 1.0 0.0 "/Game/LindwyrmRoll/Sound/SA_WyrmRumble.SA_WyrmRumble" 0))

(event EventTick
  (params (DeltaSeconds :type Float%20%28single-precision%29))
  (CallFunction|HandleRotation DeltaSeconds)
  (if (< (Variables|Default|GetTimeThrown) (Variables|Default|GetTimeOverride))
    (Variables|Default|SetTimeThrown (+ DeltaSeconds (Variables|Default|GetTimeThrown)))
    (if (Variables|Default|GetIsRolling)
      (goto _label Reset))
    (else
      (Utilities|FlowControl|DoOnce false :!label _label
        (:Completed
          (Variables|Default|SetCanFire true))))))

(fn ConstructionScript)

(fn LaunchWyrm
  (params (Direction :type Vector))
  (bind _spherehitbox (Variables|Default|GetSphereHitbox))
  (Class|PrimitiveComponent|SetAllPhysicsLinearVelocity _spherehitbox "0, 0, 0" false)
  (Class|PrimitiveComponent|SetPhysicsAngularVelocityinRadians _spherehitbox "0, 0, 0" false "None")
  (Physics|AddImpulse (Variables|Default|GetSphereHitbox) (* Direction (Variables|Default|GetImpulseStrength)) "None" true)
  (Variables|Default|SetCanFire false)
  (Variables|Default|SetTimeThrown 0.0)
  (Variables|Default|SetIsRolling true)
  (Components|Animation|PlayAnimation (Variables|Default|GetLindwyrm) "/Game/LindwyrmRoll/Characters/Lindwyrm/LindwyrmRollUp.LindwyrmRollUp" false)
  (Transformation|SetActorScale3D "3.000000,3.000000,3.000000")
  (CallFunction|TweenScale))

(fn BoostWyrm
  (bind _returnvalue (Transformation|GetVelocity))
  (if (Variables|Default|GetCanBoost)
    (Physics|AddImpulse (Variables|Default|GetSphereHitbox) (* (Class|KismetMathLibrary|VectorNormalUnsafe (Math|Vector|MakeVector (.x _returnvalue) (.y _returnvalue) 0.0)) (Variables|Default|GetBoostStrength)) "None" true)
    (bind _asbp_lindwyrm_roll_gamemode (Utilities|Casting|CastToBP_LindwyrmRollGamemode (Game|GetGameMode)))
    (Class|MinigameCapture|ApplyCameraShake (Class|MinigameBase|GetCamera _asbp_lindwyrm_roll_gamemode) 2.0 1.0)))

(fn RotateWyrmModel
  (params (A :type Float%20%28double-precision%29))
  (bind _spherehitbox (Variables|Default|GetSphereHitbox))
  (bind _returnvalue (Transformation|GetComponentVelocity _spherehitbox))
  (bind _returnvalue_2 (Class|KismetMathLibrary|VectorNormalUnsafe _returnvalue))
  (CallFunction|IncrementRotationAngle A)
  (Transformation|SetWorldRotation (Variables|Default|GetWyrm%20Pivot) (Math|Rotator|MakeRotfromZ (Math|Vector|RotateVectorAroundAxis _returnvalue_2 (Variables|Default|GetRotationAngle) (Math|Vector|CrossProduct _returnvalue_2 (Math|Vector|VectorUp)))) false false)
  (return))

(fn IncrementRotationAngle
  (params (A :type Float%20%28double-precision%29))
  (Variables|Default|SetRotationAngle (+ (* A (Variables|Default|GetRotationSpeed) (Math|Vector|VectorLength (Transformation|GetComponentVelocity (Variables|Default|GetSphereHitbox)))) (Variables|Default|GetRotationAngle))))

(fn AddRings
  (params (AmountToAdd :type Integer))
  (bind _difference (Default|SetAmountOfRings (Variables|Default|GetRingHolder) (+ AmountToAdd (Variables|/Game/LindwyrmRoll/Blueprints/Props/BP_RingHolder.BP_RingHolder_C|GetCurrentRings (Variables|Default|GetRingHolder)))))
  (return _difference))

(fn HandleRotation
  (params (Delta%20time :type Float%20%28double-precision%29))
  (if (Variables|Default|GetIsRolling)
    (CallFunction|RotateWyrmModel Delta%20time)
    (else
      (Transformation|SetRelativeRotation (Variables|Default|GetWyrm%20Pivot) "0, 0, 0" false false))))