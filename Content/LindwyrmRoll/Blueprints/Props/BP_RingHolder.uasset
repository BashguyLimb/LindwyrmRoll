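; Ring holder that displays a variable number of gold rings spaced along a spline, as a visual ring count.
; On BeginPlay it finds the spline on its owner if none is set, pre-spawns MaxRings hidden BP_GoldRing actors at even distances and attaches them to it.
; SetAmountOfRings updates the count, making each pooled ring appear or disappear by index.
; EndPlay destroys the spawned rings.
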(event EventBeginPlay
  (Variables|Default|GetRingSpline
    (:then
      _)
    (:else
      (Variables|Default|SetRingSpline (Actor|GetComponentbyClass (Components|GetOwner) "/Script/Engine.SplineComponent"))))
  (bind _output_get (Variables|Default|SetSplineLength (Spline|GetSplineLength (Variables|Default|GetRingSpline))))
  (Variables|Default|SetRingDist (/ _output_get (Variables|Default|GetMaxRings)))
  (for _index (range 0 (- (Variables|Default|GetMaxRings) 1))
    (bind _returnvalue (Game|SpawnActorfromClass "/Game/LindwyrmRoll/Blueprints/Props/BP_GoldRing.BP_GoldRing_C" (Math|Transform|MakeTransform (Spline|GetLocationatDistanceAlongSpline (Variables|Default|GetRingSpline) (* (Variables|Default|GetRingDist) _index) "World") (Spline|GetRotationatDistanceAlongSpline (Variables|Default|GetRingSpline) (* (Variables|Default|GetRingDist) _index) "World") "1.000000,1.000000,1.000000") "Undefined" (Components|GetOwner) 0))
    (Rendering|SetVisibility (Variables|/Script/Engine.Actor|GetRootComponent _returnvalue) false true)
    (Transformation|AttachComponentToComponent _returnvalue (Variables|Default|GetRingSpline) "None" "KeepWorld" "KeepWorld" "KeepWorld" true)
    (Utilities|Array|Add (Variables|Default|GetSpawnedRings) _returnvalue))
  (CallFunction|UpdateRingMeshes))

(event EventTick
  (params (DeltaSeconds :type Float%20%28single-precision%29)))

(event EventEndPlay
  (params (EndPlayReason :type EEndPlayReason%20Enum :default "Destroyed"))
  (for _array_element (Variables|Default|GetSpawnedRings)
    (Actor|DestroyActor _array_element)))

(fn SetAmountOfRings
  (params (NewAmount :type Integer))
  (Variables|Default|SetCurrentRings NewAmount)
  (CallFunction|UpdateRingMeshes))

(fn UpdateRingMeshes
  (for (_array_element _array_index) (Variables|Default|GetSpawnedRings)
    (if (< _array_index (Variables|Default|GetCurrentRings))
      (Default|OnAppear _array_element)
      (else
        (Default|OnDissapear _array_element)))))