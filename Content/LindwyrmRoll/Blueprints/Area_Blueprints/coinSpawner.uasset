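; Coin spawner actor that periodically places coins at preset point components in the level.
; BeginPlay builds the point array, which lists Coinpoint2 twice and omits Coinpoint3, then starts a looping timer that calls SpawnCoin every few seconds.
; Each SpawnCoin shuffles the array and considers the first five entries, spawning a coin only where a small sphere overlap finds no existing WorldDynamic coin.
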(event Custom|SpawnCoin
  (Utilities|Array|Shuffle (Variables|Default|GetSpawnPoints))
  (bind (_array_element _array_index) (Utilities|Array|ForEachLoopwithBreak (Variables|Default|GetSpawnPoints))
    (:LoopBody
      (if (not (> _array_index 4))
        (bind _returnvalue (Collision|SphereOverlapActors (Transformation|GetWorldLocation _array_element) 2e+01 (Utilities|Array|MakeArray "ObjectTypeQuery2") (Variables|Default|GetcoinClass)))
        (if (not _returnvalue)
          (Game|SpawnActorfromClass (Variables|Default|GetcoinClass) (Transformation|GetWorldTransform _array_element) "Undefined" 0 0))))))

(event Collision|EventActorBeginOverlap
  (params (OtherActor :type Actor%20Object%20Reference)))

(event EventTick
  (params (DeltaSeconds :type Float%20%28single-precision%29)))

(event EventBeginPlay
  (Variables|Default|SetSpawnPoints (Utilities|Array|MakeArray (Variables|Default|Getcoinpoint1) (Variables|Default|Getcoinpoint2) (Variables|Default|Getcoinpoint2) (Variables|Default|Getcoinpoint4) (Variables|Default|Getcoinpoint5) (Variables|Default|Getcoinpoint6) (Variables|Default|Getcoinpoint7) (Variables|Default|Getcoinpoint8) (Variables|Default|Getcoinpoint9) (Variables|Default|Getcoinpoint10) (Variables|Default|Getcoinpoint11) (Variables|Default|Getcoinpoint12)))
  (Utilities|Time|SetTimerbyFunctionName 0 "SpawnCoin" 3.0 true))

(fn ConstructionScript)