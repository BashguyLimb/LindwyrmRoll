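; Gold coin pickup for LindwyrmRoll that a gnome player collects by standing still inside its trigger box.
; On overlap it stores the player and starts a looping timer that checks whether they stay near the same spot, restarting the count when they move.
; After a short stay it adds gold to the player and points to their team through the game mode's point counter, then destroys itself.
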(event OnComponentBeginOverlap(TriggerBox)
  (params (OverlappedComponent :type Primitive%20Component%20Object%20Reference) (OtherActor :type Actor%20Object%20Reference) (OtherComp :type Primitive%20Component%20Object%20Reference) (OtherBodyIndex :type Integer) (bFromSweep :type Boolean) (SweepResult :type Hit%20Result%20Structure%20%28by%20ref%29))
  (bind _asbp_gnome_player (Utilities|Casting|CastToBP_GnomePlayer OtherActor))
  (Variables|Default|Set123player _asbp_gnome_player)
  (Variables|Default|SetinitalLocation (Transformation|GetActorLocation _asbp_gnome_player))
  (Variables|Default|SetisCounting true)
  (bind _returnvalue (Utilities|Time|SetTimerbyFunctionName 0 "CheckPawnMoved" 0.2 true))
  (Variables|Default|SetTimerHandle _returnvalue))

(event OnComponentEndOverlap(TriggerBox)
  (params (OverlappedComponent :type Primitive%20Component%20Object%20Reference) (OtherActor :type Actor%20Object%20Reference) (OtherComp :type Primitive%20Component%20Object%20Reference) (OtherBodyIndex :type Integer))
  (bind _asbp_gnome_player (Utilities|Casting|CastToBP_GnomePlayer OtherActor))
  (if (== _asbp_gnome_player (Variables|Default|Get123player))
    (Variables|Default|SetisCounting false)
    (Utilities|Time|ClearandInvalidateTimerbyHandle (Variables|Default|GetTimerHandle))
    (Variables|Default|Set123player 0)))

(event Custom|CheckPawnMoved
  (bind _123player (Variables|Default|Get123player))
  (bind _123player_2 (Variables|Default|Get123player))
  (bind _returnvalue (Transformation|GetActorLocation _123player))
  (if (Variables|Default|GetisCounting)
    (if (<= (Math|Vector|Distance2D(Vector) _returnvalue (Variables|Default|GetinitalLocation)) 1e+01)
      (Variables|Default|SetStayTime (+ (Variables|Default|GetStayTime) 0.2))
      (if (>= (Variables|Default|GetStayTime) 0.8)
        (Variables|/Game/LindwyrmRoll/Blueprints/GnomePlayer/BP_GnomePlayer.BP_GnomePlayer_C|SetGoldAmount _123player_2 (+ (Variables|/Game/LindwyrmRoll/Blueprints/GnomePlayer/BP_GnomePlayer.BP_GnomePlayer_C|GetGoldAmount _123player_2) 2))
        (Class|BasePointCounter|AddPoints (Class|MinigameBase|GetPointCounter (Variables|Default|GetgameMode)) (Variables|/Script/MinigameCore.MinigamePlayer|GetTeam (Variables|Default|Get123player)) 2)
        (Actor|DestroyActor)
        (Variables|Default|SetisCounting false)
        (Development|PrintText "get 2 gold!"))
      (else
        (Variables|Default|SetinitalLocation _returnvalue)
        (Variables|Default|SetStayTime 0.0)))))

(event EventBeginPlay
  (bind _asbp_lindwyrm_roll_gamemode (Utilities|Casting|CastToBP_LindwyrmRollGamemode (Game|GetGameMode)))
  (Variables|Default|SetgameMode _asbp_lindwyrm_roll_gamemode))

(event Collision|EventActorBeginOverlap
  (params (OtherActor :type Actor%20Object%20Reference)))

(event EventTick
  (params (DeltaSeconds :type Float%20%28single-precision%29)))

(fn ConstructionScript)