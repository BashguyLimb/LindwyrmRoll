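; Speed boost area that accelerates the rolling wyrm player ball when it enters.
; On trigger box overlap it casts to BP_RollingWyrm and sets the sphere hitbox's physics linear velocity to 1.5 times its current velocity as a one-off boost.
; An unconnected older path that scaled and clamped a MoveSpeed variable remains in the graph but never runs.
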(event OnComponentBeginOverlap(TigggerBox)
  (params (OverlappedComponent :type Primitive%20Component%20Object%20Reference) (OtherActor :type Actor%20Object%20Reference) (OtherComp :type Primitive%20Component%20Object%20Reference) (OtherBodyIndex :type Integer) (bFromSweep :type Boolean) (SweepResult :type Hit%20Result%20Structure%20%28by%20ref%29))
  (bind _asbp_rolling_wyrm (Utilities|Casting|CastToBP_RollingWyrm OtherActor))
  (Physics|SetPhysicsLinearVelocity (Variables|/Game/LindwyrmRoll/Blueprints/RollingWyrm/BP_RollingWyrm.BP_RollingWyrm_C|GetSphereHitbox _asbp_rolling_wyrm) (* (Transformation|GetComponentVelocity (Variables|/Game/LindwyrmRoll/Blueprints/RollingWyrm/BP_RollingWyrm.BP_RollingWyrm_C|GetSphereHitbox _asbp_rolling_wyrm)) "1.500000,1.500000,1.500000") false "None"))

(event OnComponentEndOverlap(TigggerBox)
  (params (OverlappedComponent :type Primitive%20Component%20Object%20Reference) (OtherActor :type Actor%20Object%20Reference) (OtherComp :type Primitive%20Component%20Object%20Reference) (OtherBodyIndex :type Integer)))

(event EventBeginPlay)

(event Collision|EventActorBeginOverlap
  (params (OtherActor :type Actor%20Object%20Reference)))

(event EventTick
  (params (DeltaSeconds :type Float%20%28single-precision%29)))

(fn ConstructionScript)