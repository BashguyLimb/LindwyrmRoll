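; BP_123player is the player pawn for the 123 minigame, with movement, death and respawn.
; BeginPlay resets the PlayerRotation component, caches the BP_123Gamemode from Minigame and records the start location.
; IA_Movement drives movement input along control-rotation axes, scaled by MoveSpeed.
; Die, guarded by IsDead, resets MoveSpeed and disables input, then after RebirthTime calls Rebirth to return the player to the start and restore input.
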(event Custom|Die
  (params (rebirthTime :type Float%20%28double-precision%29))
  (if (not (Variables|Default|GetisDead))
    (Variables|Default|SetisDead true)
    (Variables|Default|SetMoveSpeed 1.0)
    (Input|DisableInput 0)
    (Utilities|FlowControl|Delay rebirthTime)
    (CallFunction|Rebirth)))

(event Custom|Rebirth
  (Transformation|SetActorLocation (Variables|Default|GetstartPosition) false false)
  (Input|EnableInput 0)
  (Variables|Default|SetisDead false))

(event Input|EnhancedActionEvents|EnhancedInputActionIA_Movement
  (params (ActionValue :type Vector%202D%20Structure) (ElapsedSeconds :type Float%20%28double-precision%29) (TriggeredSeconds :type Float%20%28double-precision%29) (InputAction :type Input%20Action%20Object%20Reference :default "/MinigameCore/Input/IA_Movement.IA_Movement"))
  (bind (_x _y) (Math|Vector2D|BreakVector2D ActionValue))
  (:Triggered
    (Pawn|Input|AddMovementInput (Math|Vector|GetRightVector (Pawn|GetControlRotation :!class /Script/Engine.Pawn)) (* (Variables|Default|GetMoveSpeed) _x) false)
    (Pawn|Input|AddMovementInput (Math|Vector|GetForwardVector (Pawn|GetControlRotation :!class /Script/Engine.Pawn)) (* (Variables|Default|GetMoveSpeed) _y) false)))

(event EventBeginPlay
  (Class|PlayerRotationComponent|ResetInitialOrientation (Variables|Default|GetPlayerRotation))
  (bind _asbp_123gamemode (Utilities|Casting|CastToBP_123Gamemode (Variables|Default|GetMinigame)))
  (Variables|Default|Set123game _asbp_123gamemode)
  (Variables|Default|SetstartPosition (Transformation|GetActorLocation)))

(event Collision|EventActorBeginOverlap
  (params (OtherActor :type Actor%20Object%20Reference)))

(event EventTick
  (params (DeltaSeconds :type Float%20%28single-precision%29)))

(fn ConstructionScript)