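; AI controller that drives a BP_GnomePlayer in the LindwyrmRoll minigame.
; On possession it caches the gnome, then loops AI moves to random reachable points within a radius around it, pausing briefly after each successful move.
; The loop has no failure branch, so a failed move ends the wandering.
; Independently, Tick makes the gnome jump whenever CanJump is true.
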(event Custom|Mover
  (bind _as_bp_gnome_player (Variables|Default|GetAs%20BP%20Gnome%20Player))
  (bind _as_bp_gnome_player_2 (Variables|Default|GetAs%20BP%20Gnome%20Player))
  (bind _returnvalue (Transformation|GetActorRotation _as_bp_gnome_player))
  (AI|AIMoveTo _as_bp_gnome_player_2 (.RandomLocation (AI|Navigation|GetRandomReachablePointinRadius (Transformation|GetWorldLocation (Variables|/Script/Engine.Actor|GetRootComponent _as_bp_gnome_player_2)) 1e+03 0 0)) 0 5.0 false
    (:OnSuccess
      (Transformation|SetActorRotation (Variables|Default|GetAs%20BP%20Gnome%20Player) (Math|Interpolation|RInterpTo _returnvalue (Math|Conversions|RotationFromXVector (Math|Vector|GetForwardVector _returnvalue)) 0.0 0.0))
      (Utilities|FlowControl|Delay 2.0)
      (CallFunction|Mover))))

(event EventOnMinigamePlayerPossessed
  (bind _asbp_gnome_player (Utilities|Casting|CastToBP_GnomePlayer (Variables|Default|GetPlayer)))
  (bind _output_get (Variables|Default|SetAs%20BP%20Gnome%20Player _asbp_gnome_player))
  (CallFunction|Mover))

(event EventTick
  (params (DeltaSeconds :type Float%20%28single-precision%29))
  (if (Variables|/Game/LindwyrmRoll/Blueprints/GnomePlayer/BP_GnomePlayer.BP_GnomePlayer_C|GetCanJump (stale EventOnMinigamePlayerPossessed _output_get))
    (Default|Jump (stale EventOnMinigamePlayerPossessed _output_get))))

(fn ConstructionScript)