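; AI controller for computer-controlled players in the Lindwyrm Roll minigame.
; On possession it caches the BP_RollingPlayer, then each tick raises CurrentRotation while below MaxRotation and lowers it otherwise.
; With no direction state, the rotation climbs to the maximum and jitters there rather than sweeping back.
; A random one-in-three ThrowWyrm call, gated by CanFire, is present but disconnected, so the AI never throws.
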(event EventOnMinigamePlayerPossessed
  (bind _asbp_rolling_player (Utilities|Casting|CastToBP_RollingPlayer (Variables|Default|GetPlayer)))
  (Variables|Default|SetAs%20BP%20Rolling%20Player _asbp_rolling_player))

(event EventTick
  (params (DeltaSeconds :type Float%20%28single-precision%29))
  (bind _as_bp_rolling_player (Variables|Default|GetAs%20BP%20Rolling%20Player))
  (if (< (Variables|/Game/LindwyrmRoll/Blueprints/RollingPlayer/BP_RollingPlayer.BP_RollingPlayer_C|GetCurrent%20Rotation _as_bp_rolling_player) (Variables|/Game/LindwyrmRoll/Blueprints/RollingPlayer/BP_RollingPlayer.BP_RollingPlayer_C|GetMaxRotation _as_bp_rolling_player))
    (CallFunction|Increment)
    (else
      (CallFunction|Decrement))))

(fn ConstructionScript)

(fn Increment
  (bind _as_bp_rolling_player (Variables|Default|GetAs%20BP%20Rolling%20Player))
  (bind _result (Math|Float|IncrementFloat (Variables|/Game/LindwyrmRoll/Blueprints/RollingPlayer/BP_RollingPlayer.BP_RollingPlayer_C|GetCurrent%20Rotation _as_bp_rolling_player))
    (:%20%20
      (Variables|/Game/LindwyrmRoll/Blueprints/RollingPlayer/BP_RollingPlayer.BP_RollingPlayer_C|SetCurrent%20Rotation _as_bp_rolling_player _result))))

(fn Decrement
  (bind _as_bp_rolling_player (Variables|Default|GetAs%20BP%20Rolling%20Player))
  (bind _result (Math|Float|DecrementFloat (Variables|/Game/LindwyrmRoll/Blueprints/RollingPlayer/BP_RollingPlayer.BP_RollingPlayer_C|GetCurrent%20Rotation _as_bp_rolling_player))
    (:%20%20
      (Variables|/Game/LindwyrmRoll/Blueprints/RollingPlayer/BP_RollingPlayer.BP_RollingPlayer_C|SetCurrent%20Rotation _as_bp_rolling_player _result))))