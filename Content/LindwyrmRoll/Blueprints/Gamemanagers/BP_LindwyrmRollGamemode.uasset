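; Game mode for LindwyrmRoll that manages a two-team score between Gnomes and Rollers through a PointCounter.
; On begin play and reset, it gives the Gnomes their default points and zeroes the Rollers; begin play also starts banjo music.
; TransferPointsToRollers moves points from the Gnome pool to the Rollers, crediting them with the absolute amount.
; Debug prints remain in begin play and the transfer.
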(event EventBeginPlay
  (|CallParentFunction)
  (CallFunction|SetDefaultPoints)
  (Audio|PlaySound2D "/Game/LindwyrmRoll/Sound/Heftone_Banjo_Orchestra_-_Dill_Pickles.Heftone_Banjo_Orchestra_-_Dill_Pickles" 1.0 1.0 0.0 0 0)
  (Development|PrintString "Hello"))

(event EventTick
  (params (DeltaSeconds :type Float%20%28single-precision%29))
  (|CallParentFunction DeltaSeconds) ; This node is disabled and will not be called.\nDrag off pins to build functionality.
)

(event EventOnReset
  (|CallParentFunction)
  (CallFunction|SetDefaultPoints))

(fn ConstructionScript
  (|CallParentFunction))

(fn SetDefaultPoints
  (Class|BasePointCounter|SetPoints (Variables|Default|GetPoint%20Counter) 1 (Variables|Default|GetDefaultGnomePoints))
  (Class|BasePointCounter|SetPoints (Variables|Default|GetPoint%20Counter))
  (return))

(fn TransferPointstoRollers
  (params (Amount :type Integer))
  (bind _result (Utilities|NegateInt Amount)
    (:%20%20
      (Class|BasePointCounter|AddPoints (Variables|Default|GetPoint%20Counter) 1 _result)
      (Development|PrintString (Utilities|String|ToString(Integer) Amount))
      (Class|BasePointCounter|AddPoints (Variables|Default|GetPoint%20Counter) 0 (Math|Integer|Absolute(Integer) Amount)))))