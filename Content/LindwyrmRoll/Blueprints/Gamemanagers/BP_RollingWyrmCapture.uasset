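; BP_RollingWyrmCapture is an actor in LindwyrmRoll that holds an unfinished camera-shake setup.
; BeginPlay stores the start position and casts to the LindwyrmRoll game mode without using the result, while Tick only advances a shake timer.
; The Perlin-noise offset around the start position is unused, the shake event is empty, and the binding and shake calls never run, so the actor never moves.
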(event Custom|TriggerCameraShake_Event
  (params (Duration :type Float%20%28double-precision%29) (Amplitude :type Vector) (Frequency :type Float%20%28double-precision%29)))

(event EventBeginPlay
  (|CallParentFunction)
  (Variables|Default|SetStartPosition (Transformation|GetActorLocation))
  (Utilities|Casting|CastToBP_LindwyrmRollGamemode (Game|GetGameMode)))

(event EventTick
  (params (DeltaSeconds :type Float%20%28single-precision%29))
  (bind _output_get (Variables|Default|SetTime (+ (* DeltaSeconds (Variables|Default|GetShakeSpeed)) (Variables|Default|GetTime)))))

(fn ConstructionScript
  (|CallParentFunction))